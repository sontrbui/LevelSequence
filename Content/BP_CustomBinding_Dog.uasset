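; BP_CustomBinding_Dog is a Sequencer custom binding that swaps the player pawn for a placed dog character at runtime.
; On resolve, it takes the first actor tagged ReplacePlayer, casts it to BP_DogCharacter and has the first player controller possess it.
; The dog moves to the old pawn's transform, the old pawn is destroyed, and the dog is returned as the bound object.
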(fn `BP_ResolveRuntimeBinding`
  (params (ResolveContext :type "MovieSceneBindingResolveContext Structure (by ref)"))
  (returns (ReturnValue :type "MovieSceneBindingResolveResult Structure"))
  (locals (OldPlayerPawn :type "Pawn Object Reference") (NewPawn :type "/Game/Characters/Cow/BP_DogCharacter Object Reference"))
  (bind _returnvalue (`GameplayStatics.GetPlayerController` ResolveContext_WorldContext))
  (bind _outactors (`GameplayStatics.GetAllActorsWithTag` ResolveContext_WorldContext "ReplacePlayer"))
  (bind _asbp_dog_character (cast `/Game/Characters/Cow/BP_DogCharacter` (`|GetArrayItem` _outactors)))
  (bind _output_get (set `local.OldPlayerPawn` (`GameplayStatics.GetPlayerPawn` _returnvalue)))
  (bind _output_get_2 (set `local.NewPawn` _asbp_dog_character))
  (`Controller.Possess` _returnvalue _output_get_2)
  (`Actor.K2_SetActorTransform` _output_get_2 (`Actor.GetTransform` _output_get) false false)
  (`Actor.K2_DestroyActor` _output_get)
  (return (make `MovieSceneBindingResolveResult` (`|MakeArray` _output_get_2 :!type "Object Object Reference"))))